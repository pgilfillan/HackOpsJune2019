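; BP_CharacterBase is a base Blueprint for flat characters that handles switching between alive and dead states.
; OnDeath clears IsAlive, shows the death icon, hides the speech bubble and plays a 2D death sound.
; OnAlive reverses the state and visual changes for un-dying during time rewind.
; Both events print the character's name with a status message, and nothing in this graph calls them.
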(event `self.ReceiveBeginPlay`)

(event `OnDeath`
  (`KismetSystemLibrary.PrintString` (`KismetStringLibrary.Concat_StrStr` (`KismetSystemLibrary.GetDisplayName` null) " died"))
  (set `self.IsAlive` false)
  (`SceneComponent.SetVisibility` (`self.DeathIcon`) true false)
  (`SceneComponent.SetVisibility` (`self.SpeechBubble`) false false)
  (`GameplayStatics.PlaySound2D` (`self.DeathSoundCue`) 1.0 1.0 0.0 null null))

(event `OnAlive`
  (`KismetSystemLibrary.PrintString` (`KismetStringLibrary.Concat_StrStr` (`KismetSystemLibrary.GetDisplayName` null) " recovers"))
  (set `self.IsAlive` true)
  (`SceneComponent.SetVisibility` (`self.DeathIcon`) false false)
  (`SceneComponent.SetVisibility` (`self.SpeechBubble`) true false))

(fn `UserConstructionScript`)