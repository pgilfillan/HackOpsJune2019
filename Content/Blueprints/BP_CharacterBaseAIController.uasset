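; AI controller that sends its pawn to randomly chosen target points as part of a simulation.
; On possess, it caches all TargetPoint actors and the first BP_SimulationController in the level.
; GoTo_Event picks a random target via ChooseTarget and runs AIMoveTo toward its location.
; Success calls CharacterFinishAction on the simulation controller, while failure only prints a debug message.
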(event `self.ReceivePossess`
  (params (PossessedPawn :type "Pawn Object Reference"))
  (bind _outactors (`GameplayStatics.GetAllActorsOfClass` "/Script/Engine.TargetPoint"))
  (set `self.TargetArray` _outactors)
  (bind _outactors_2 (`GameplayStatics.GetAllActorsOfClass` "/Game/Blueprints/BP_SimulationController.BP_SimulationController_C"))
  (set `self.SimulationController` (`|GetArrayItem` _outactors_2)))

(event `GoTo_Event`
  (bind _newparam (`self.ChooseTarget`))
  (`/Engine/EditorBlueprintResources/StandardMacros.IsValid` _newparam
    (:`Is Valid`
      (bind _movementresult (`|AIMoveTo` (`self.K2_GetPawn`) (`self.K2_GetActorLocation` _newparam) null 5.0 true)
        (:`OnSuccess`
          (`/Game/Blueprints/BP_SimulationController.CharacterFinishAction` (`self.SimulationController`)))
        (:`OnFail`
          (`KismetSystemLibrary.PrintString` (`KismetStringLibrary.Concat_StrStr` (`KismetSystemLibrary.GetDisplayName` (`self.K2_GetPawn`)) " failed to move " (`|GetEnumeratorNameAsString` _movementresult))))))))

(fn `ChooseTarget`
  (returns (NewParam :type "TargetPoint Object Reference"))
  (bind _output_get (set `self.CurrentTarget` (`|GetArrayItem` (`self.TargetArray`) (`KismetMathLibrary.RandomIntegerInRange` 0 (- (`KismetArrayLibrary.Array_Length` (`self.TargetArray`)) 1)))))
  (`KismetSystemLibrary.PrintString` (`KismetStringLibrary.Concat_StrStr` (`KismetSystemLibrary.GetDisplayName` (`self.K2_GetPawn`)) "'s target is " (`KismetSystemLibrary.GetDisplayName` _output_get)))
  (return _output_get))

(fn `UserConstructionScript`)