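; Simulation controller that seeds the world state and starts a turn for the AI characters.
; BeginPlay builds the state from a seed plus character, room and item lists, then fires GoToEvent on every character AI controller.
; A counter resets once all characters report finishing, but no next turn is wired.
; SetMapFromState, not called here, teleports characters to TargetPoints matched to their state room by name.
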(event `StartTurn`
  (bind _outactors (`GameplayStatics.GetAllActorsOfClass` "/Game/Blueprints/BP_CharacterBaseAIController.BP_CharacterBaseAIController_C"))
  (for _array_element _outactors
    (`/Game/Blueprints/BP_CharacterBaseAIController.GoTo_Event` _array_element)))

(event `self.ReceiveBeginPlay`
  (bind _returnvalue (`self.ResetSimulationState` (`self.Seed`) (`self.CharacterNames`) (`self.CharacterBPs`) (`self.RoomNames`) (`self.RoomLocations`) (`self.ItemNames`) (`self.ItemBPs`)))
  (`self.StartTurn`)
  (set `self.CurrentMapState` _returnvalue))

(event `CharacterFinishAction`
  (bind _result (`/Engine/EditorBlueprintResources/StandardMacros.IncrementInt` (`self.CharactersFinishActionCount`))
    (:`  `
      (`/Engine/EditorBlueprintResources/StandardMacros.CompareInt` (`KismetArrayLibrary.Array_Length` (`self.CharacterNames`)) _result
        (:`==`
          (set `self.CharactersFinishActionCount` 0))))))

(fn `SetMapFromState`
  (params (State :type "MapState Structure"))
  (bind _outactors (`GameplayStatics.GetAllActorsOfClass` "/Game/Blueprints/3dCharacters/3dCharacterBase.3dCharacterBase_C"))
  (for _array_element _outactors
    (bind _returnvalue (`self.GetRoomNameForCharacter` State (`KismetSystemLibrary.GetObjectName` _array_element)))
    (bind _outactors_2 (`GameplayStatics.GetAllActorsOfClass` "/Script/Engine.TargetPoint"))
    (for _array_element_2 _outactors_2
      (if (== (`KismetStringLibrary.Replace` (`KismetSystemLibrary.GetDisplayName` _array_element_2) "TargetPoint") _returnvalue)
        (`self.K2_TeleportTo` _array_element (`self.K2_GetActorLocation` _array_element_2) (`self.K2_GetActorRotation` _array_element))))))

(fn `UserConstructionScript`)