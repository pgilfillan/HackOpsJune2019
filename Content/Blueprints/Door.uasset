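; Clickable door actor that links two named rooms in a simulation and toggles between open and closed.
; On click it flips IsOpen and passes the new state and both room names to the first BP_SimulationController found, against its current map state.
; It then applies a dynamic instance of the open or closed material and teleports down when opening, back up when closing.
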(event `self.ReceiveActorOnClicked`
  (params (ButtonPressed :type "Key Structure"))
  (bind _staticmeshcomponent (`self.StaticMeshComponent`))
  (bind _staticmeshcomponent_2 (`self.StaticMeshComponent`))
  (bind _output_get (set `self.IsOpen` (not (`self.IsOpen`))))
  (bind _outactors (`GameplayStatics.GetAllActorsOfClass` "/Game/Blueprints/BP_SimulationController.BP_SimulationController_C"))
  (bind _output (`|GetArrayItem` _outactors))
  (`SimulationController.ChangeDoorOpen` _output (`/Game/Blueprints/BP_SimulationController.CurrentMapState` _output) (`self.Room1`) (`self.Room2`) _output_get)
  (if _output_get
    (bind _returnvalue (`PrimitiveComponent.CreateDynamicMaterialInstance` _staticmeshcomponent_2 0 "/Game/Textures/OpenDoor_Mat.OpenDoor_Mat" "None"))
    (`PrimitiveComponent.SetMaterial` _staticmeshcomponent_2 0 _returnvalue)
    (`self.K2_SetActorLocation` (+ (`self.K2_GetActorLocation`) (0.0 0.0 -40.0)) false true)
    (else
      (bind _returnvalue_2 (`PrimitiveComponent.CreateDynamicMaterialInstance` _staticmeshcomponent 0 "/Game/Textures/ClosedDoor_Mat.ClosedDoor_Mat" "None"))
      (`PrimitiveComponent.SetMaterial` _staticmeshcomponent 0 _returnvalue_2)
      (`self.K2_SetActorLocation` (+ (`self.K2_GetActorLocation`) (0.0 0.0 40.0)) false true))))

(fn `UserConstructionScript`)